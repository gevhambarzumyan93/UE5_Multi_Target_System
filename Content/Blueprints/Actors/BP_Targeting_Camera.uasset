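; Targeting camera rig that frames its owner (the player) and a target.
; On BeginPlay it spawns a camera actor on its spring arm and makes it the player's view.
; Custom events set clamped zoom, turn the camera toward the owner and update field of view.
; FOV is the law-of-cosines angle between player and target at the camera, padded and clamped; C_Focus is the older coordinate-based version.
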(event Custom|C_Zoom
  (params (Arm%20Length :type Float%20%28single-precision%29))
  (Variables|/Script/Engine.SpringArmComponent|SetTargetArmLength (Variables|Default|GetSpringArm) (Math|Float|Clamp(Float) Arm%20Length 8e+02 2.5e+03)))

(event Custom|C_RotateCamera
  (bind _returnvalue (Components|GetOwner))
  (if (Utilities|IsValid _returnvalue)
    (Transformation|SetActorRotation (Variables|Default|GetTargetCamera) (Math|Rotator|FindLookatRotation (Transformation|GetActorLocation (Variables|Default|GetTargetCamera)) (Transformation|GetActorLocation _returnvalue)))))

(event Custom|C_Focus
  (params (PlayerCord :type Vector) (TargetCord :type Vector))
  ;[1 0 0.3072] old version (still working but unnecessary)
  (Camera|SetFieldOfView (Variables|/Game/Blueprints/Actors/BP_Camera_Actor.BP_Camera_Actor_C|GetCamera (Variables|Default|GetTargetCamera)) (Math|Float|Clamp(Float) (+ (CallFunction|CalcCameraViewAngle PlayerCord TargetCord) (Variables|Default|GetExtraAngle)) 9e+01 1.2e+02)))

(event Custom|C_Update_Field_Of_View
  (params (InTarget :type Actor%20Object%20Reference))
  (Camera|SetFieldOfView (Variables|/Game/Blueprints/Actors/BP_Camera_Actor.BP_Camera_Actor_C|GetCamera (Variables|Default|GetTargetCamera)) (Math|Float|Clamp(Float) (+ (CallFunction|CalcCameraFieldOfView InTarget) (Variables|Default|GetExtraAngle)) 9e+01 1.2e+02)))

(event EventBeginPlay
  (bind _returnvalue (Game|SpawnActorfromClass "/Game/Blueprints/Actors/BP_Camera_Actor.BP_Camera_Actor_C" (Variables|Default|GetSpawn%20Transform) "Undefined" 0 0))
  (bind _output_get (Variables|Default|SetTargetCamera _returnvalue))
  (Transformation|AttachComponentToComponent _output_get (Variables|Default|GetSpringArm) "None" "KeepRelative" "KeepRelative" "KeepRelative" true)
  (Game|Player|SetViewTargetwithBlend (Game|GetPlayerController 0) (Variables|Default|GetTargetCamera) 0.0 "VTBlend_Linear" 0.0 false))

(fn ConstructionScript)

(fn CalcCameraViewAngle
  (params (PlayerCord :type Vector) (TargetCord :type Vector))
  (bind _targetcamera (Variables|Default|GetTargetCamera))
  (bind _targetcamera_2 (Variables|Default|GetTargetCamera))
  (bind _returnvalue (Transformation|GetActorLocation _targetcamera_2))
  (bind _returnvalue_2 (Transformation|GetActorLocation _targetcamera))
  (Utilities|FlowControl|Sequence
    (:then_0
      (LocalVariables|SetDistancePlayerToTarget (Utilities|CalcDistance (.x PlayerCord) (.y PlayerCord) (.z PlayerCord) (.x TargetCord) (.y TargetCord) (.z TargetCord))))
    (:then_1
      (LocalVariables|SetDistanceTargetToCamera (Utilities|CalcDistance (.x _returnvalue) (.y _returnvalue) (.z _returnvalue) (.x TargetCord) (.y TargetCord) (.z TargetCord))))
    (:then_2
      (LocalVariables|SetDistancePlayerToCamera (Utilities|CalcDistance (.x _returnvalue_2) (.y _returnvalue_2) (.z _returnvalue_2) (.x PlayerCord) (.y PlayerCord) (.z PlayerCord))))
    (:then_3
      (return (* (Math|Trig|Acos(Degrees) (/ (- (+ (Math|Float|Power (LocalVariables|GetDistancePlayerToCamera) 2.0) (Math|Float|Power (LocalVariables|GetDistanceTargetToCamera) 2.0)) (Math|Float|Power (LocalVariables|GetDistancePlayerToTarget) 2.0)) (* 2.0 (LocalVariables|GetDistancePlayerToCamera) (LocalVariables|GetDistanceTargetToCamera)))) (/ 1.8e+02 (Math|Trig|GetPI)))))))

(fn CalcCameraFieldOfView
  (params (Target :type Actor%20Object%20Reference))
  (Utilities|FlowControl|Sequence
    (:then_0
      (LocalVariables|SetDistancePlayerToTarget (Transformation|GetDistanceTo Target (Components|GetOwner))))
    (:then_1
      (LocalVariables|SetDistanceTargetToCamera (Transformation|GetDistanceTo (Variables|Default|GetTargetCamera) Target)))
    (:then_2
      (LocalVariables|SetDistancePlayerToCamera (Transformation|GetDistanceTo (Variables|Default|GetTargetCamera) (Components|GetOwner))))
    (:then_3
      (return (* (Math|Trig|Acos(Degrees) (/ (- (+ (Math|Float|Power (LocalVariables|GetDistancePlayerToCamera) 2.0) (Math|Float|Power (LocalVariables|GetDistanceTargetToCamera) 2.0)) (Math|Float|Power (LocalVariables|GetDistancePlayerToTarget) 2.0)) (* 2.0 (LocalVariables|GetDistancePlayerToCamera) (LocalVariables|GetDistanceTargetToCamera)))) (/ 1.8e+02 (Math|Trig|GetPI)))))))