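; Lock-on targeting component that locks its owner onto a nearby actor and drives a separate targeting camera.
; Enabling lock-on sphere-traces around the owner for a target, then spawns BP_Targeting_Camera and fires a summon event.
; Tick lerps the camera in XY toward the owner-target midpoint, offset toward the owner at long range, and zooms by clamped distance.
; Toggling off or reaching MaxDistance clears the target and destroys the camera.
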(event Custom|C_EnableLockOn
  (bind (_retrunvalue _target) (Targeting|FindTarget))
  (if _retrunvalue
    (Variables|Default|SetTarget _target)
    (CallFunction|SetIsTargeting true)
    (Camera|SummonTargetCamera)))

(event Custom|C_DisableLockOn
  (Variables|Default|SetTarget 0)
  (CallFunction|SetIsTargeting false)
  (Camera|DestroyCamera))

(event Custom|C_ToggleLockOn
  (if (not (Variables|Default|GetIsTargeting))
    (CallFunction|CEnableLockon)
    (else
      (CallFunction|CDisableLockon))))

(event EventTick
  (params (DeltaSeconds :type Float%20%28single-precision%29))
  (bind (_x _y) (Helper|LerpCords))
  (bind _target (Variables|Default|GetTarget))
  (bind _returnvalue (Transformation|GetActorLocation _target))
  (bind _returnvalue_2 (Targeting|CalcDistancetoTarget _returnvalue))
  (if (Variables|Default|GetIsTargeting)
    (Camera|UpdateTargetCameraLocation _x _y)
    (Default|CZoom (Variables|Default|GetTargetCamera) (Math|Float|Clamp(Float) _returnvalue_2 1e+02 1e+03))
    (if (>= _returnvalue_2 (Variables|Default|GetMaxDistance))
      (CallFunction|CDisableLockon))))

(fn SetIsTargeting
  (params (EnableTargeting :type Boolean))
  (Variables|Default|SetIsTargeting EnableTargeting))

(fn GetIsTargeting
  (return (Variables|Default|GetIsTargeting)))

(fn FindTarget
  (bind _returnvalue (Components|GetOwner))
  (bind _returnvalue_2 (Transformation|GetActorLocation _returnvalue))
  (bind (_outhit _returnvalue_3) (Collision|SphereTraceForObjects _returnvalue_2 _returnvalue_2 (Variables|Default|GetTargetingDistance) (Variables|Default|GetTarget%20Object%20Types) false (Utilities|Array|MakeArray (Components|GetOwner)) "ForDuration"))
  (if (and _returnvalue_3 (Utilities|IsValid (.HitActor (Collision|BreakHitResult _outhit))))
    (return true (.HitActor (Collision|BreakHitResult _outhit)))
    (else
      (return false 0))))

(fn GetTarget
  (return (Variables|Default|GetTarget)))

(fn CalcTargetingPoint
  (bind _returnvalue (Components|GetOwner))
  (bind _target (Variables|Default|GetTarget))
  (bind _returnvalue_2 (Transformation|GetActorLocation _target))
  (bind _returnvalue_3 (Transformation|GetActorLocation _returnvalue))
  (LocalVariables|SetNewLocation (/ (+ (Transformation|GetActorLocation (Components|GetOwner)) _returnvalue_2) 2))
  (if (< (Targeting|CalcDistancetoTarget _returnvalue_2) 1.5e+03)
    (return (LocalVariables|GetNewLocation))
    (else
      (Development|PrintString "mtav")
      (LocalVariables|SetDeltaX (- (.x (LocalVariables|GetNewLocation)) (.x _returnvalue_3)))
      (LocalVariables|SetDeltaY (- (.y (LocalVariables|GetNewLocation)) (.y _returnvalue_3)))
      (return (Math|Vector|MakeVector (- (.x (LocalVariables|GetNewLocation)) (.PointDeltaX (Helper|GetDeltaCord (LocalVariables|GetDeltaX) (LocalVariables|GetDeltaY) 2e+01 (* (Targeting|CalcDistancetoTarget (Transformation|GetActorLocation (Variables|Default|GetTarget))) 0.01)))) (- (.y (LocalVariables|GetNewLocation)) (.PointDeltaY (Helper|GetDeltaCord (LocalVariables|GetDeltaX) (LocalVariables|GetDeltaY) 2e+01 (* (Targeting|CalcDistancetoTarget (Transformation|GetActorLocation (Variables|Default|GetTarget))) 0.01)))) 0.0)))))

(fn SummonTargetCamera
  (bind _returnvalue (Targeting|CalcTargetingPoint))
  (bind _returnvalue_2 (Game|SpawnActorfromClass "/Game/Blueprints/Actors/BP_Targeting_Camera.BP_Targeting_Camera_C" (Math|Transform|MakeTransform (Math|Vector|MakeVector (.x _returnvalue) (.y _returnvalue) 1e+02) "0, 0, 0" "1.000000,1.000000,1.000000") "Undefined" 0 0))
  (Variables|Default|SetTargetCamera _returnvalue_2)
  (Default|CallOnCameraSummon))

(fn DestroyCamera
  (Actor|DestroyActor (Variables|Default|GetTargetCamera))
  (Default|CallOnCameraDestroy))

(fn UpdateTargetCameraLocation
  (params (XCord :type Float%20%28double-precision%29) (YCord :type Float%20%28double-precision%29))
  (bind _targetcamera (Variables|Default|GetTargetCamera))
  (bind _rootcomponent (Variables|/Script/Engine.Actor|GetRootComponent _targetcamera))
  (if (not (and (Utilities|Check XCord (Variables|Default|GetLastX)) (Utilities|Check YCord (Variables|Default|GetLastY))))
    (Variables|Default|SetLastX XCord)
    (Variables|Default|SetLastY YCord)
    (Transformation|SetWorldLocation _rootcomponent (Math|Vector|MakeVector (Variables|Default|GetLastX) (Variables|Default|GetLastY) (.z (Transformation|GetWorldLocation _rootcomponent))) false false)))

(fn CalcDistancetoTarget
  (params (TargetVector :type Vector))
  (return (Math|Vector|Distance(Vector) TargetVector (Transformation|GetActorLocation (Components|GetOwner)))))

(fn FindMinorMaxValue
  (params (Value :type Float%20%28double-precision%29) (Min :type Float%20%28double-precision%29) (Max :type Float%20%28double-precision%29))
  (if (< Value Min)
    (return true Value)
    (else
      (return false (Math|Float|Max(Float) Max Value)))))

(fn GetDeltaCord
  (params (DeltaX :type Float%20%28double-precision%29) (DeltaY :type Float%20%28double-precision%29) (DeltaStep :type Float%20%28double-precision%29) (StepLength :type Float%20%28double-precision%29))
  (LocalVariables|SetLength (Math|Float|Sqrt (+ (Math|Float|Power DeltaX 2.0) (Math|Float|Power DeltaY 2.0))))
  (return (* (* (/ DeltaX (LocalVariables|GetLength)) DeltaStep) StepLength) (* StepLength (* DeltaStep (/ DeltaY (LocalVariables|GetLength))))))

(fn LerpCords
  (if (< (+ (/ (Utilities|Time|GetWorldDeltaSeconds) 1e+02) (Variables|Default|GetAlpha)) 0.9)
    (Variables|Default|SetAlpha (+ (/ (Utilities|Time|GetWorldDeltaSeconds) 1e+02) (Variables|Default|GetAlpha)))
    (else
      (Variables|Default|SetAlpha 0.0)))
  (return (Math|Float|Lerp (Variables|Default|GetLastX) (.x (Targeting|CalcTargetingPoint)) (Math|Float|Clamp(Float) (Variables|Default|GetAlpha))) (Math|Float|Lerp (Variables|Default|GetLastY) (.y (Targeting|CalcTargetingPoint)) (Math|Float|Clamp(Float) (Variables|Default|GetAlpha)))))