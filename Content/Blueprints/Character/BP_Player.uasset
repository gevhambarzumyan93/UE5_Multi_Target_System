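; Player Blueprint that handles Enhanced Input movement and target lock-on.
; BeginPlay adds the player mapping context, and the move action applies input along fixed world X/Y axes rather than relative to camera or control rotation.
; Lock-on toggles through the BPC_Targeting_V2 component, while the older BPC_Targeting toggle is left unconnected.
; Both targeting components' camera-destroy events blend the view target back to the player.
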(event OnCameraDestroy(BPC_Targeting_V2)
  (Game|Player|SetViewTargetwithBlend (Game|GetPlayerController 0) self 0.0 "VTBlend_Linear" 0.0 false))

(event OnCameraDestroy(BPC_Targeting)
  (Game|Player|SetViewTargetwithBlend (Game|GetPlayerController 0) self 0.0 "VTBlend_Linear" 0.0 false))

(event Input|EnhancedActionEvents|EnhancedInputActionIA_Move
  (params (ActionValue :type Vector%202D%20Structure) (ElapsedSeconds :type Float%20%28double-precision%29) (TriggeredSeconds :type Float%20%28double-precision%29) (InputAction :type Input%20Action%20Object%20Reference :default "/Game/Blueprints/Character/Inputs/IA_Move.IA_Move"))
  (:Triggered
    (Pawn|Input|AddMovementInput "0.0,1.000000,0.0" (.x ActionValue) false)
    (Pawn|Input|AddMovementInput "1.000000,0.000000,0.000000" (.y ActionValue) false)))

(event Input|EnhancedActionEvents|EnhancedInputActionIA_Lock_On
  (params (ActionValue :type Boolean) (ElapsedSeconds :type Float%20%28double-precision%29) (TriggeredSeconds :type Float%20%28double-precision%29) (InputAction :type Input%20Action%20Object%20Reference :default "/Game/Blueprints/Character/Inputs/IA_Lock_On.IA_Lock_On"))
  (:Started
    (Default|CToggleLockon (Variables|Default|GetBPC_Targeting_V2))))

(event EventBeginPlay
  (bind _asplayer_controller (Utilities|Casting|CastToPlayerController (Pawn|GetController)))
  (Utilities|IsValid (PlayerController|LocalPlayerSubsystems|GetEnhancedInputLocalPlayerSubsystem _asplayer_controller)
    (:Is%20Valid
      (Input|AddMappingContext (PlayerController|LocalPlayerSubsystems|GetEnhancedInputLocalPlayerSubsystem _asplayer_controller) "/Game/Blueprints/Character/Inputs/IMC_Player.IMC_Player" 0 "(bIgnoreAllPressedKeysUntilRelease=True,bForceImmediately=False)"))))

(fn ConstructionScript)